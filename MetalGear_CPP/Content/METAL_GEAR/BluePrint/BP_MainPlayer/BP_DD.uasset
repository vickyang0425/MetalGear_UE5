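; BP_DD is the DD character Blueprint in the main-player folder, handling its montage playback and movement state.
; Tick caches whether the movement component is falling.
; A PlayMontage event stores an upper-slot-only flag, plays the montage on the mesh and, if interrupted, calls CallEventDispatcherForAttackInterrupt.
; The construction script records the spring arm's relative height as original and current camera height.
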(event Custom|PlayMontage
  (params (UppperOrDefault :type Boolean) (Montage :type Anim%20Montage%20Object%20Reference))
  (Utilities|FlowControl|Sequence
    (:then_0
      (Variables|Default|SetisOnlyUseUpperSlot_DD UppperOrDefault)
      (Animation|Montage|PlayMontage (Variables|Character|GetMesh) Montage
        (:OnInterrupted
          (Default|CallEventDispatcherforAttackInterrupt))))))

(event EventBeginPlay)

(event EventTick
  (params (DeltaSeconds :type Float%20%28single-precision%29))
  (Variables|Default|SetisFalling_DD (AI|Components|NavMovement|IsFalling (Variables|Character|GetCharacterMovement))))

(fn ConstructionScript
  (bind _springarm (Variables|Default|GetSpringArm))
  (bind _relativelocation (Variables|/Script/Engine.SceneComponent|GetRelativeLocation _springarm))
  (Variables|aboutCrouchCamera|SetOriginalCameraHeight (.z _relativelocation))
  (Variables|aboutCrouchCamera|SetCurrentCameraHeight (.z _relativelocation)))