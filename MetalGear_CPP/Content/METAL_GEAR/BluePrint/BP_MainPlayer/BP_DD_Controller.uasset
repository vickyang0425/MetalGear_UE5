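; Player controller for the DD character that turns Enhanced Input into movement, auto-move, crouch, jump, dash, roll, attacks, combos and weapon equip.
; Can-functions gate actions on character state flags, which AnimBlueprint event dispatchers set as montages hit start, end and weapon-swap points.
; Equip and sword attack montages switch to upper-body versions while moving, airborne or crouched.
; Crouching resizes the capsule and eases the spring arm height with a timeline.
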(event Custom|UpdateCameraHeight
  (bind _bp_dd_ref (Variables|Default|GetBP_DD_Ref))
  (bind _bp_dd_ref_2 (Variables|Default|GetBP_DD_Ref))
  (bind _bp_dd_ref_3 (Variables|Default|GetBP_DD_Ref))
  (bind _springarm (Variables|/Game/Metal_Gear/BluePrint/BP_MainPlayer/BP_DD.BP_DD_C|GetSpringArm _bp_dd_ref_2))
  (bind _relativelocation (Variables|/Script/Engine.SceneComponent|GetRelativeLocation _springarm))
  ;[1 1 1] 下蹲镜头缓慢更新
  (Utilities|FlowControl|Sequence
    (:then_0
      (if (Variables|/Game/Metal_Gear/BluePrint/BP_MainPlayer/BP_DD.BP_DD_C|GethasCrouch_DD (Variables|Default|GetBP_DD_Ref))
        (Variables|/Game/Metal_Gear/BluePrint/BP_MainPlayer/BP_DD.BP_DD_C|SetTargetCameraHeight (Variables|Default|GetBP_DD_Ref) 4e+01)
        (CallFunction|SetCharactorCapsuleSize 6e+01 -27.0)
        (else
          (Variables|/Game/Metal_Gear/BluePrint/BP_MainPlayer/BP_DD.BP_DD_C|SetTargetCameraHeight (Variables|Default|GetBP_DD_Ref) 1.2e+02)
          (CallFunction|SetCharactorCapsuleSize 4e+01 0.0))))
    (:then_2
      ;;[1 1 1] 如果当前高度和目标高度不一致的话说明发生了下蹲，用ori先把current的记录下来。再让cur从ori缓慢变成target
      (if (!= (Variables|/Game/Metal_Gear/BluePrint/BP_MainPlayer/BP_DD.BP_DD_C|GetTargetCameraHeight _bp_dd_ref_3) (Variables|/Game/Metal_Gear/BluePrint/BP_MainPlayer/BP_DD.BP_DD_C|GetCurrentCameraHeight _bp_dd_ref_3))
        (Variables|/Game/Metal_Gear/BluePrint/BP_MainPlayer/BP_DD.BP_DD_C|SetOriginalCameraHeight _bp_dd_ref (Variables|/Game/Metal_Gear/BluePrint/BP_MainPlayer/BP_DD.BP_DD_C|GetCurrentCameraHeight _bp_dd_ref))
        (bind _crouchcachetime (Timeline|CrouchUpDown PlayFromStart)
          (:Update
            (Transformation|SetRelativeLocation _springarm (Math|Vector|MakeVector (.x _relativelocation) (.y _relativelocation) (Math|Float|Lerp (Variables|/Game/Metal_Gear/BluePrint/BP_MainPlayer/BP_DD.BP_DD_C|GetOriginalCameraHeight _bp_dd_ref_2) (Variables|/Game/Metal_Gear/BluePrint/BP_MainPlayer/BP_DD.BP_DD_C|GetTargetCameraHeight _bp_dd_ref_2) _crouchcachetime)) false false)
            ;;[1 1 1] timeline每过一帧更新一次
            (Variables|/Game/Metal_Gear/BluePrint/BP_MainPlayer/BP_DD.BP_DD_C|SetCurrentCameraHeight (Variables|Default|GetBP_DD_Ref) (Math|Float|Lerp (Variables|/Game/Metal_Gear/BluePrint/BP_MainPlayer/BP_DD.BP_DD_C|GetOriginalCameraHeight _bp_dd_ref_2) (Variables|/Game/Metal_Gear/BluePrint/BP_MainPlayer/BP_DD.BP_DD_C|GetTargetCameraHeight _bp_dd_ref_2) _crouchcachetime))))))))

(event Custom|CusEvent_OnEquipGotWeapon
  (bind _bp_dd_ref (Variables|Default|GetBP_DD_Ref))
  ;[1 1 1 1 15] 动画蓝图传过来的拿武器的事件分发器，并逻辑运行后面连接的自定义event，把是否拿武器bool设为true
  (Variables|/Game/Metal_Gear/BluePrint/BP_MainPlayer/BP_DD.BP_DD_C|SethasWeapons_DD _bp_dd_ref true)
  (Transformation|AttachComponentToComponent (Variables|/Game/Metal_Gear/BluePrint/BP_MainPlayer/BP_DD.BP_DD_C|GetSword _bp_dd_ref) (Variables|/Script/Engine.Character|GetMesh _bp_dd_ref) "AAA" "KeepRelative" "KeepRelative" "KeepRelative" true))

(event Custom|CusEvent_UnequipEnd
  ;[1 1 1] 注释
  (Variables|/Game/Metal_Gear/BluePrint/BP_MainPlayer/BP_DD.BP_DD_C|SetisUnequiping_DD (Variables|Default|GetBP_DD_Ref) false))

(event Custom|CusEvent_OnAttackInterrupt
  ;[1 1 1] 攻击打断
  ;;[1 1 1] Cus
  (Variables|/Game/Metal_Gear/BluePrint/BP_MainPlayer/BP_DD.BP_DD_C|SetisAttacking (Variables|Default|GetBP_DD_Ref) false))

(event Custom|CusEvent_OnComboStart
  ;[1 1 1] 连招
  (Variables|/Game/Metal_Gear/BluePrint/BP_MainPlayer/BP_DD.BP_DD_C|SetisComboing (Variables|Default|GetBP_DD_Ref) true))

(event Custom|CusEvent_OnComboEnd
  ;[1 1 1] 连招
  (Variables|/Game/Metal_Gear/BluePrint/BP_MainPlayer/BP_DD.BP_DD_C|SetisComboing (Variables|Default|GetBP_DD_Ref) false))

(event Custom|CusEvent_OnUnequipBackWeapon
  (bind _bp_dd_ref (Variables|Default|GetBP_DD_Ref))
  ;[1 1 1] 注释
  (Variables|/Game/Metal_Gear/BluePrint/BP_MainPlayer/BP_DD.BP_DD_C|SethasWeapons_DD _bp_dd_ref false)
  (Transformation|AttachComponentToComponent (Variables|/Game/Metal_Gear/BluePrint/BP_MainPlayer/BP_DD.BP_DD_C|GetSword _bp_dd_ref) (Variables|/Script/Engine.Character|GetMesh _bp_dd_ref) "Sword_2" "KeepRelative" "KeepRelative" "KeepRelative" true))

(event Custom|CusEvent_OnAttackStart
  (Variables|/Game/Metal_Gear/BluePrint/BP_MainPlayer/BP_DD.BP_DD_C|SetisAttacking (Variables|Default|GetBP_DD_Ref) true))

(event Custom|CusEvent_OnShiftingStart
  ;[1 1 1] shift设置
  (Variables|/Game/Metal_Gear/BluePrint/BP_MainPlayer/BP_DD.BP_DD_C|SetisShifting (Variables|Default|GetBP_DD_Ref) true))

(event Custom|CusEvent_OnAttackEnd
  (Variables|/Game/Metal_Gear/BluePrint/BP_MainPlayer/BP_DD.BP_DD_C|SetisAttacking (Variables|Default|GetBP_DD_Ref) false))

(event Custom|CusEvent_OnShiftingEnd
  ;[1 1 1] shift设置
  (Variables|/Game/Metal_Gear/BluePrint/BP_MainPlayer/BP_DD.BP_DD_C|SetisShifting (Variables|Default|GetBP_DD_Ref) false))

(event Custom|CusEvent_EquipStart
  ;[1 1 1 1 15] 动画蓝图传过来的拿武器的事件分发器，并逻辑运行后面连接的自定义event，把是否拿武器bool设为true
  (Variables|/Game/Metal_Gear/BluePrint/BP_MainPlayer/BP_DD.BP_DD_C|SetisEquiping_DD (Variables|Default|GetBP_DD_Ref) true))

(event Custom|CusEvent_EquipEnd
  ;[1 1 1 1 15] 动画蓝图传过来的拿武器的事件分发器，并逻辑运行后面连接的自定义event，把是否拿武器bool设为true
  (Variables|/Game/Metal_Gear/BluePrint/BP_MainPlayer/BP_DD.BP_DD_C|SetisEquiping_DD (Variables|Default|GetBP_DD_Ref) false))

(event Custom|CusEvent_UnequipStart
  ;[1 1 1] 注释
  (Variables|/Game/Metal_Gear/BluePrint/BP_MainPlayer/BP_DD.BP_DD_C|SetisUnequiping_DD (Variables|Default|GetBP_DD_Ref) true))

(event Input|EnhancedActionEvents|EnhancedInputActionIA_Jump
  (params (ActionValue :type Boolean) (ElapsedSeconds :type Float%20%28double-precision%29) (TriggeredSeconds :type Float%20%28double-precision%29) (InputAction :type Input%20Action%20Object%20Reference :default "/Game/Metal_Gear/EnhancedInput/IA_Jump.IA_Jump"))
  (bind _bp_dd_ref (Variables|Default|GetBP_DD_Ref))
  ;[1 1 1] ue5本身就不支持蹲下时，可以跳跃，这个需要自己写
  (:Started
    (bind _flag (CallFunction|CanJump))
    (if _flag
      (Character|Jump _bp_dd_ref)))
  (:Completed
    (Character|StopJumping _bp_dd_ref)))

(event Input|EnhancedActionEvents|EnhancedInputActionIA_LookUpAndDown
  (params (ActionValue :type Float%20%28double-precision%29) (ElapsedSeconds :type Float%20%28double-precision%29) (TriggeredSeconds :type Float%20%28double-precision%29) (InputAction :type Input%20Action%20Object%20Reference :default "/Game/Metal_Gear/EnhancedInput/IA_LookUpAndDown.IA_LookUpAndDown"))
  (:Triggered
    (Pawn|Input|AddControllerPitchInput (Variables|Default|GetBP_DD_Ref) ActionValue)))

(event Input|EnhancedActionEvents|EnhancedInputActionIA_GeneralAttack
  (params (ActionValue :type Boolean) (ElapsedSeconds :type Float%20%28double-precision%29) (TriggeredSeconds :type Float%20%28double-precision%29) (InputAction :type Input%20Action%20Object%20Reference :default "/Game/Metal_Gear/EnhancedInput/IA_GeneralAttack.IA_GeneralAttack"))
  ;[1 1 1] 普攻
  (:Started
    (bind _flag (CallFunction|CanAttack？))
    (if _flag
      (CallFunction|DoGeneralAttack))))

(event Input|EnhancedActionEvents|EnhancedInputActionIA_EquipOrUnequipWeapon
  (params (ActionValue :type Boolean) (ElapsedSeconds :type Float%20%28double-precision%29) (TriggeredSeconds :type Float%20%28double-precision%29) (InputAction :type Input%20Action%20Object%20Reference :default "/Game/Metal_Gear/EnhancedInput/IA_EquipOrUnequipWeapon.IA_EquipOrUnequipWeapon"))
  ;[1 1 1] 装备武器和卸载武器
  (:Started
    (bind _flag (CallFunction|CanEquiporUnequipWeapon))
    (if _flag
      (CallFunction|EquiporUnequipWeapon))))

(event Input|EnhancedActionEvents|EnhancedInputActionIA_ComboA
  (params (ActionValue :type Boolean) (ElapsedSeconds :type Float%20%28double-precision%29) (TriggeredSeconds :type Float%20%28double-precision%29) (InputAction :type Input%20Action%20Object%20Reference :default "/Game/Metal_Gear/EnhancedInput/IA_ComboA.IA_ComboA"))
  ;[1 1 1] 普攻连击A
  (:Started
    (bind _flag (CallFunction|CanComboAttack))
    (if _flag
      (Default|PlayMontage (Variables|Default|GetBP_DD_Ref) false "/Game/Metal_Gear/DD/Animations/Montages/Attack/RootMotion/Attack_Combo_01.Attack_Combo_01"))))

(event Input|EnhancedActionEvents|EnhancedInputActionIA_ComboB
  (params (ActionValue :type Boolean) (ElapsedSeconds :type Float%20%28double-precision%29) (TriggeredSeconds :type Float%20%28double-precision%29) (InputAction :type Input%20Action%20Object%20Reference :default "/Game/Metal_Gear/EnhancedInput/IA_ComboB.IA_ComboB"))
  ;[1 1 1] 普攻连击B
  (:Started
    (bind _flag (CallFunction|CanComboAttack))
    (if _flag
      (Default|PlayMontage (Variables|Default|GetBP_DD_Ref) false "/Game/Metal_Gear/DD/Animations/Montages/Attack/RootMotion/Attack_Combo_02.Attack_Combo_02"))))

(event Input|EnhancedActionEvents|EnhancedInputActionIA_TurnRightAndLeft
  (params (ActionValue :type Float%20%28double-precision%29) (ElapsedSeconds :type Float%20%28double-precision%29) (TriggeredSeconds :type Float%20%28double-precision%29) (InputAction :type Input%20Action%20Object%20Reference :default "/Game/Metal_Gear/EnhancedInput/IA_TurnRightAndLeft.IA_TurnRightAndLeft"))
  (:Triggered
    (Pawn|Input|AddControllerYawInput (Variables|Default|GetBP_DD_Ref) ActionValue)))

(event Input|EnhancedActionEvents|EnhancedInputActionIA_MoveForwardAndBack
  (params (ActionValue :type Float%20%28double-precision%29) (ElapsedSeconds :type Float%20%28double-precision%29) (TriggeredSeconds :type Float%20%28double-precision%29) (InputAction :type Input%20Action%20Object%20Reference :default "/Game/Metal_Gear/EnhancedInput/IA_MoveForwardAndBack.IA_MoveForwardAndBack"))
  (bind _bp_dd_ref (Variables|Default|GetBP_DD_Ref))
  (:Triggered
    (Variables|/Game/Metal_Gear/BluePrint/BP_MainPlayer/BP_DD.BP_DD_C|SetisAutoMoving_DD _bp_dd_ref false)
    (Pawn|Input|AddMovementInput _bp_dd_ref (Math|Vector|GetForwardVector (Math|Rotator|MakeRotator 0.0 0.0 (.yaw (Transformation|GetActorRotation (Game|GetPlayerController 0))))) ActionValue false)))

(event Input|EnhancedActionEvents|EnhancedInputActionIA_MoveRightAndLeft
  (params (ActionValue :type Float%20%28double-precision%29) (ElapsedSeconds :type Float%20%28double-precision%29) (TriggeredSeconds :type Float%20%28double-precision%29) (InputAction :type Input%20Action%20Object%20Reference :default "/Game/Metal_Gear/EnhancedInput/IA_MoveRightAndLeft.IA_MoveRightAndLeft"))
  (bind _bp_dd_ref (Variables|Default|GetBP_DD_Ref))
  (:Triggered
    (Variables|/Game/Metal_Gear/BluePrint/BP_MainPlayer/BP_DD.BP_DD_C|SetisAutoMoving_DD _bp_dd_ref false)
    (Pawn|Input|AddMovementInput _bp_dd_ref (Math|Vector|GetRightVector (Math|Rotator|MakeRotator 0.0 0.0 (.yaw (Transformation|GetActorRotation (Game|GetPlayerController 0))))) ActionValue false)))

(event Input|EnhancedActionEvents|EnhancedInputActionIA_Crouch
  (params (ActionValue :type Boolean) (ElapsedSeconds :type Float%20%28double-precision%29) (TriggeredSeconds :type Float%20%28double-precision%29) (InputAction :type Input%20Action%20Object%20Reference :default "/Game/Metal_Gear/EnhancedInput/IA_Crouch.IA_Crouch"))
  (bind _bp_dd_ref (Variables|Default|GetBP_DD_Ref))
  ;[1 1 1] 蹲下起立
  (:Started
    (Utilities|FlowControl|FlipFlop
      (:A
        (Character|Crouch _bp_dd_ref)
        (CallFunction|DoCrouching))
      (:B
        (Character|UnCrouch _bp_dd_ref)
        (CallFunction|DoCrouching)))
    (CallFunction|UpdateCameraHeight)))

(event Input|EnhancedActionEvents|EnhancedInputActionIA_isWalk
  (params (ActionValue :type Boolean) (ElapsedSeconds :type Float%20%28double-precision%29) (TriggeredSeconds :type Float%20%28double-precision%29) (InputAction :type Input%20Action%20Object%20Reference :default "/Game/Metal_Gear/EnhancedInput/IA_isWalk.IA_isWalk"))
  ;[1 1 1] 走和跑之间的转换
  (:Started
    (CallFunction|DoWalking)))

(event Input|EnhancedActionEvents|EnhancedInputActionIA_AutoMove
  (params (ActionValue :type Boolean) (ElapsedSeconds :type Float%20%28double-precision%29) (TriggeredSeconds :type Float%20%28double-precision%29) (InputAction :type Input%20Action%20Object%20Reference :default "/Game/Metal_Gear/EnhancedInput/IA_AutoMove.IA_AutoMove"))
  (bind _bp_dd_ref (Variables|Default|GetBP_DD_Ref))
  ;[1 1 1] 是否自动移动
  (:Started
    (bind _flag (CallFunction|CanAutoMove))
    (if _flag
      (Variables|/Game/Metal_Gear/BluePrint/BP_MainPlayer/BP_DD.BP_DD_C|SetisAutoMoving_DD _bp_dd_ref (not (Variables|/Game/Metal_Gear/BluePrint/BP_MainPlayer/BP_DD.BP_DD_C|GetisAutoMoving_DD _bp_dd_ref))))))

(event Input|EnhancedActionEvents|EnhancedInputActionIA_Sprint
  (params (ActionValue :type Boolean) (ElapsedSeconds :type Float%20%28double-precision%29) (TriggeredSeconds :type Float%20%28double-precision%29) (InputAction :type Input%20Action%20Object%20Reference :default "/Game/Metal_Gear/EnhancedInput/IA_Sprint.IA_Sprint"))
  ;[1 1 1] 向前冲刺
  (:Started
    (bind _flag (CallFunction|CanShift))
    (if _flag
      (Default|PlayMontage (Variables|Default|GetBP_DD_Ref) false "/Game/Metal_Gear/DD/Animations/Montages/Montage_Dash.Montage_Dash"))))

(event Input|EnhancedActionEvents|EnhancedInputActionIA_RollingForward
  (params (ActionValue :type Boolean) (ElapsedSeconds :type Float%20%28double-precision%29) (TriggeredSeconds :type Float%20%28double-precision%29) (InputAction :type Input%20Action%20Object%20Reference :default "/Game/Metal_Gear/EnhancedInput/IA_RollingForward.IA_RollingForward"))
  ;[1 1 1] 向前翻滚
  (:Started
    (bind _flag (CallFunction|CanShift))
    (if _flag
      (Default|PlayMontage (Variables|Default|GetBP_DD_Ref) false "/Game/Metal_Gear/DD/Animations/Montages/Montage_Rolling_Front.Montage_Rolling_Front"))))

(event EventBeginPlay
  (bind _self self)
  (bind _returnvalue (PlayerController|LocalPlayerSubsystems|GetEnhancedInputLocalPlayerSubsystem _self))
  (Utilities|FlowControl|Sequence
    (:then_0
      (bind _asbp_dd (Utilities|Casting|CastToBP_DD (Game|GetPlayerCharacter 0)))
      (bind _output_get (Variables|Default|SetBP_DD_Ref _asbp_dd))
      (bind _assk_dd_skeleton_anim_blueprint (Utilities|Casting|CastToSK_DD_Skeleton_AnimBlueprint (Components|SkeletalMesh|GetAnimInstance (Variables|/Script/Engine.Character|GetMesh _output_get))))
      (Variables|Default|SetABP_DD_Ref _assk_dd_skeleton_anim_blueprint))
    (:then_1
      (Input|AddMappingContext _returnvalue "/Game/Metal_Gear/EnhancedInput/IMC_BaseMotion.IMC_BaseMotion" 0 "(bIgnoreAllPressedKeysUntilRelease=True,bForceImmediately=False)")
      (Input|AddMappingContext _returnvalue "/Game/Metal_Gear/EnhancedInput/IMC_OtherMotion.IMC_OtherMotion" 0 "(bIgnoreAllPressedKeysUntilRelease=True,bForceImmediately=False)")
      (Input|AddMappingContext _returnvalue "/Game/Metal_Gear/EnhancedInput/IMC_GeneralAttack.IMC_GeneralAttack" 0 "(bIgnoreAllPressedKeysUntilRelease=True,bForceImmediately=False)"))
    (:then_2
      ;[1 1 1 1 15] 动画蓝图传过来的拿武器的事件分发器，并逻辑运行后面连接的自定义event，把是否拿武器bool设为true
      (EventDispatchers|BindEventtoABPEventDispatcherforEquipStart (Variables|Default|GetABP_DD_Ref) (delegate Custom|CusEvent_EquipStart))
      (EventDispatchers|BindEventtoABPEventDispatcherforEquipGotWeapon (Variables|Default|GetABP_DD_Ref) (delegate Custom|CusEvent_OnEquipGotWeapon))
      (EventDispatchers|BindEventtoABPEventDispatcherforEquipEnd (Variables|Default|GetABP_DD_Ref) (delegate Custom|CusEvent_EquipEnd)))
    (:then_3
      ;[1 1 1] 注释
      (EventDispatchers|BindEventtoABPEventDispatcherforUnequipStart (Variables|Default|GetABP_DD_Ref) (delegate Custom|CusEvent_UnequipStart))
      (EventDispatchers|BindEventtoABPEventDispatcherforUnequipBackWeapon (Variables|Default|GetABP_DD_Ref) (delegate Custom|CusEvent_OnUnequipBackWeapon))
      (EventDispatchers|BindEventtoABPEventDispatcherforUnequipEnd (Variables|Default|GetABP_DD_Ref) (delegate Custom|CusEvent_UnequipEnd)))
    (:then_4
      ;[1 1 1] shift设置
      (EventDispatchers|BindEventtoABPEventDispatcherforShiftStart (Variables|Default|GetABP_DD_Ref) (delegate Custom|CusEvent_OnShiftingStart))
      (EventDispatchers|BindEventtoABPEventDispatcherforShiftEnd (Variables|Default|GetABP_DD_Ref) (delegate Custom|CusEvent_OnShiftingEnd))
      (EventDispatchers|BindEventtoABPEventDispatcherforAttackStart (Variables|Default|GetABP_DD_Ref) (delegate Custom|CusEvent_OnAttackStart))
      (EventDispatchers|BindEventtoABPEventDispatcherforAttackEnd (Variables|Default|GetABP_DD_Ref) (delegate Custom|CusEvent_OnAttackEnd)))
    (:then_5
      ;[1 1 1] 连招
      (EventDispatchers|BindEventtoABPEventDispatcherforComboStart (Variables|Default|GetABP_DD_Ref) (delegate Custom|CusEvent_OnComboStart))
      (EventDispatchers|BindEventtoABPEventDispatcherforComboEnd (Variables|Default|GetABP_DD_Ref) (delegate Custom|CusEvent_OnComboEnd)))
    (:then_6
      ;[1 1 1] 攻击打断
      (EventDispatchers|BindEventtoEventDispatcherforAttackInterrupt (Variables|Default|GetBP_DD_Ref) (delegate Custom|CusEvent_OnAttackInterrupt)))))

(event EventTick
  (params (DeltaSeconds :type Float%20%28single-precision%29))
  (bind _bp_dd_ref (Variables|Default|GetBP_DD_Ref))
  (Utilities|FlowControl|Sequence
    (:then_0
      ;[1 1 1] 执行一直移动
      (if (Variables|/Game/Metal_Gear/BluePrint/BP_MainPlayer/BP_DD.BP_DD_C|GetisAutoMoving_DD _bp_dd_ref)
        (Pawn|Input|AddMovementInput _bp_dd_ref (Transformation|GetActorForwardVector (Game|GetPlayerCharacter 0)) 1.0 false)))
    (:then_1
      (Development|PrintString (Utilities|String|ToString(Boolean) (Variables|/Game/Metal_Gear/BluePrint/BP_MainPlayer/BP_DD.BP_DD_C|GetisComboing (Variables|Default|GetBP_DD_Ref)))))))

(fn ConstructionScript)

(fn SetCharactorCapsuleSize
  (params (CapsuleRadius :type Float%20%28double-precision%29) (MeshRelativeLocationX :type Float%20%28double-precision%29))
  (bind _bp_dd_ref (Variables|Default|GetBP_DD_Ref))
  (bind _mesh (Variables|/Script/Engine.Character|GetMesh _bp_dd_ref))
  (bind _returnvalue (Transformation|GetRelativeTransform _mesh))
  (Components|Capsule|SetCapsuleRadius (Variables|/Script/Engine.Character|GetCapsuleComponent _bp_dd_ref) CapsuleRadius true)
  (Transformation|SetRelativeTransform _mesh (Math|Transform|MakeTransform (Math|Vector|MakeVector MeshRelativeLocationX (.y (.location _returnvalue)) (.z (.location _returnvalue))) (.rotation _returnvalue) (.scale _returnvalue)) false false))

(fn DoWalking
  (bind _bp_dd_ref (Variables|Default|GetBP_DD_Ref))
  (bind _bp_dd_ref_2 (Variables|Default|GetBP_DD_Ref))
  (bind _charactermovement (Variables|/Script/Engine.Character|GetCharacterMovement _bp_dd_ref_2))
  ;[1 1 1] 二话不说先把走路状态改变
  (bind _output_get (Variables|/Game/Metal_Gear/BluePrint/BP_MainPlayer/BP_DD.BP_DD_C|SetisWalking_DD _bp_dd_ref (not (Variables|/Game/Metal_Gear/BluePrint/BP_MainPlayer/BP_DD.BP_DD_C|GetisWalking_DD _bp_dd_ref))))
  ;[1 1 1] 如果是走路，和不是走路
  (if _output_get
    (Variables|/Script/Engine.CharacterMovementComponent|SetMaxWalkSpeed _charactermovement (Variables|/Game/Metal_Gear/BluePrint/BP_MainPlayer/BP_DD.BP_DD_C|GetWalkGroundSpeed _bp_dd_ref_2))
    (else
      (Variables|/Script/Engine.CharacterMovementComponent|SetMaxWalkSpeed _charactermovement (Variables|/Game/Metal_Gear/BluePrint/BP_MainPlayer/BP_DD.BP_DD_C|GetRunGroundSpeed _bp_dd_ref_2)))))

(fn DoCrouching
  (bind _bp_dd_ref (Variables|Default|GetBP_DD_Ref))
  (bind _output_get (Variables|/Game/Metal_Gear/BluePrint/BP_MainPlayer/BP_DD.BP_DD_C|SethasCrouch_DD _bp_dd_ref (not (Variables|/Game/Metal_Gear/BluePrint/BP_MainPlayer/BP_DD.BP_DD_C|GethasCrouch_DD _bp_dd_ref))))
  (if _output_get
    _))

(fn DoJumping)

(fn DoPlayMontage
  (params (Montage :type Anim%20Montage%20Object%20Reference) (IsOnlyUseUpperSlot :type Boolean))
  (bind _bp_dd_ref (Variables|Default|GetBP_DD_Ref))
  (Utilities|FlowControl|Sequence
    (:then_0
      (Animation|PlayAnimMontage _bp_dd_ref Montage 1.0 "default"))
    (:then_1
      (Variables|/Game/Metal_Gear/BluePrint/BP_MainPlayer/BP_DD.BP_DD_C|SetisOnlyUseUpperSlot_DD _bp_dd_ref IsOnlyUseUpperSlot))))

(fn DoGeneralAttack
  (bind _bp_dd_ref (Variables|Default|GetBP_DD_Ref))
  (bind _abp_dd_ref (Variables|Default|GetABP_DD_Ref))
  (bind _charactermovement (Variables|/Script/Engine.Character|GetCharacterMovement _bp_dd_ref))
  (bind _groundspeed (Variables|/Game/Metal_Gear/BluePrint/BP_MainPlayer/SK_DD_Skeleton_AnimBlueprint.SK_DD_Skeleton_AnimBlueprint_C|GetGroundSpeed _abp_dd_ref))
  (bind _returnvalue (AI|Components|NavMovement|IsCrouching _charactermovement))
  (bind _returnvalue_2 (AI|Components|NavMovement|IsFalling _charactermovement))
  (bind _returnvalue_3 (> _groundspeed 0.0))
  (bind _returnvalue_4 (Math|Boolean|ORBoolean _returnvalue_2 _returnvalue _returnvalue_3))
  (if (Variables|/Game/Metal_Gear/BluePrint/BP_MainPlayer/BP_DD.BP_DD_C|GethasWeapons_DD (Variables|Default|GetBP_DD_Ref))
    (if _returnvalue_4
      ;[1 1 1] 如果手上有武器，且人物在空中或者移动就播放可融合的普攻montage
      (Default|PlayMontage (Variables|Default|GetBP_DD_Ref) true "/Game/Metal_Gear/DD/Animations/Montages/Attack/InPlace/Attack_02_UpperBody.Attack_02_UpperBody")
      (else
        (Default|PlayMontage (Variables|Default|GetBP_DD_Ref) false "/Game/Metal_Gear/DD/Animations/Montages/Attack/InPlace/Attack_02.Attack_02")))
    (else
      ;[1 1 1] 是否移动的时候播放装备攻击
      (if _returnvalue_4
        _
        (else
          _))
      ;[1 1 1] 没移动播放不需要融合的
      (Default|PlayMontage (Variables|Default|GetBP_DD_Ref) false "/Game/Metal_Gear/DD/Animations/Montages/Attack/RootMotion/Attack_Eqip_01.Attack_Eqip_01"))))

(fn DoAttachWeapon)

(fn EquiporUnequipWeapon
  (bind _bp_dd_ref (Variables|Default|GetBP_DD_Ref))
  (bind _abp_dd_ref (Variables|Default|GetABP_DD_Ref))
  (bind _charactermovement (Variables|/Script/Engine.Character|GetCharacterMovement _bp_dd_ref))
  (bind _groundspeed (Variables|/Game/Metal_Gear/BluePrint/BP_MainPlayer/SK_DD_Skeleton_AnimBlueprint.SK_DD_Skeleton_AnimBlueprint_C|GetGroundSpeed _abp_dd_ref))
  (bind _returnvalue (AI|Components|NavMovement|IsCrouching _charactermovement))
  (bind _returnvalue_2 (AI|Components|NavMovement|IsFalling _charactermovement))
  (bind _returnvalue_3 (> _groundspeed 0.0))
  (bind _returnvalue_4 (Math|Boolean|ORBoolean _returnvalue_2 _returnvalue _returnvalue_3))
  ;[1 1 1 1 12] 如果有武器按下R就是卸下武器，没武器按下R就是装备武器
  (if (Variables|/Game/Metal_Gear/BluePrint/BP_MainPlayer/BP_DD.BP_DD_C|GethasWeapons_DD (Variables|Default|GetBP_DD_Ref))
    ;[1 1 1] true就播放融合的；false播放不融合的
    (if _returnvalue_4
      (Default|PlayMontage (Variables|Default|GetBP_DD_Ref) true "/Game/Metal_Gear/DD/Animations/Montages/Eqip_To_Uneqip_UpperBody.Eqip_To_Uneqip_UpperBody")
      (else
        (Default|PlayMontage (Variables|Default|GetBP_DD_Ref) false "/Game/Metal_Gear/DD/Animations/Montages/Eqip_To_Uneqip.Eqip_To_Uneqip")))
    (else
      ;[1 1 1] true就播放融合的；false播放不融合的
      (if _returnvalue_4
        (Default|PlayMontage (Variables|Default|GetBP_DD_Ref) true "/Game/Metal_Gear/DD/Animations/Montages/Uneqip_To_Eqip_UpperBody.Uneqip_To_Eqip_UpperBody")
        (else
          (Default|PlayMontage (Variables|Default|GetBP_DD_Ref) false "/Game/Metal_Gear/DD/Animations/Montages/Uneqip_To_Eqip.Uneqip_To_Eqip"))))))

(fn UnequipWeapon)

(fn CanAttack？
  (bind _bp_dd_ref (Variables|Default|GetBP_DD_Ref))
  (bind _bp_dd_ref_2 (Variables|Default|GetBP_DD_Ref))
  (Utilities|FlowControl|Sequence
    (:then_0
      ;[1 1 1 1 13] 已经播放攻击montage了就不能再播放了除非结束当前播放
      (if (Variables|/Game/Metal_Gear/BluePrint/BP_MainPlayer/BP_DD.BP_DD_C|GetisAttacking _bp_dd_ref_2)
        (Development|PrintString "已经正在攻击，不能攻击，必须等当前攻击播放完")
        (return false)))
    (:then_1
      (if (Variables|/Game/Metal_Gear/BluePrint/BP_MainPlayer/BP_DD.BP_DD_C|GetisEquiping_DD _bp_dd_ref_2)
        (Development|PrintString "正在装备武器不能攻击")
        (return false)))
    (:then_2
      (if (Variables|/Game/Metal_Gear/BluePrint/BP_MainPlayer/BP_DD.BP_DD_C|GetisUnequiping_DD _bp_dd_ref)
        (Development|PrintString "正在卸载武器不能攻击")
        (return false)))
    (:then_4
      (if (Variables|/Game/Metal_Gear/BluePrint/BP_MainPlayer/BP_DD.BP_DD_C|GetisShifting _bp_dd_ref)
        (Development|PrintString "正在冲刺或翻滚不能攻击")
        (return false)))
    (:then_5
      (return true))))

(fn CanComboAttack
  (bind _flag (CallFunction|CanAttack？))
  (if _flag
    ;[1 1 1 1 13] 手上没武器也不能连环攻击
    (if (Variables|/Game/Metal_Gear/BluePrint/BP_MainPlayer/BP_DD.BP_DD_C|GethasWeapons_DD (Variables|Default|GetBP_DD_Ref))
      (return true)
      (else
        (Development|PrintString "手上没武器不能连击")
        (return false)))
    (else
      (return false))))

(fn CanMove)

(fn CanEquiporUnequipWeapon
  (bind _bp_dd_ref (Variables|Default|GetBP_DD_Ref))
  (if (Math|Boolean|ORBoolean (Variables|/Game/Metal_Gear/BluePrint/BP_MainPlayer/BP_DD.BP_DD_C|GetisUnequiping_DD _bp_dd_ref) (Variables|/Game/Metal_Gear/BluePrint/BP_MainPlayer/BP_DD.BP_DD_C|GetisEquiping_DD _bp_dd_ref) (Variables|/Game/Metal_Gear/BluePrint/BP_MainPlayer/BP_DD.BP_DD_C|GetisAttacking _bp_dd_ref) (Variables|/Game/Metal_Gear/BluePrint/BP_MainPlayer/BP_DD.BP_DD_C|GetisShifting _bp_dd_ref))
    (return false)
    (else
      (return true))))

(fn CanAutoMove
  (bind _bp_dd_ref (Variables|Default|GetBP_DD_Ref))
  (if (or (Variables|/Game/Metal_Gear/BluePrint/BP_MainPlayer/BP_DD.BP_DD_C|GetisEquiping_DD _bp_dd_ref) (Variables|/Game/Metal_Gear/BluePrint/BP_MainPlayer/BP_DD.BP_DD_C|GetisUnequiping_DD _bp_dd_ref))
    (return false)
    (else
      (return true))))

(fn CanShift
  (bind _bp_dd_ref (Variables|Default|GetBP_DD_Ref))
  (if (Math|Boolean|ORBoolean (Variables|/Game/Metal_Gear/BluePrint/BP_MainPlayer/BP_DD.BP_DD_C|GetisShifting _bp_dd_ref) (Variables|/Game/Metal_Gear/BluePrint/BP_MainPlayer/BP_DD.BP_DD_C|GetisComboing _bp_dd_ref) (Variables|/Game/Metal_Gear/BluePrint/BP_MainPlayer/BP_DD.BP_DD_C|GetisFalling_DD _bp_dd_ref) (Variables|/Game/Metal_Gear/BluePrint/BP_MainPlayer/BP_DD.BP_DD_C|GetisEquiping_DD _bp_dd_ref) (Variables|/Game/Metal_Gear/BluePrint/BP_MainPlayer/BP_DD.BP_DD_C|GetisUnequiping_DD _bp_dd_ref))
    (return false)
    (else
      (return true))))

(fn CanJump
  (bind _bp_dd_ref (Variables|Default|GetBP_DD_Ref))
  (if (or (Variables|/Game/Metal_Gear/BluePrint/BP_MainPlayer/BP_DD.BP_DD_C|GetisComboing _bp_dd_ref) (Variables|/Game/Metal_Gear/BluePrint/BP_MainPlayer/BP_DD.BP_DD_C|GetisShifting _bp_dd_ref))
    (return false)
    (else
      (return true))))